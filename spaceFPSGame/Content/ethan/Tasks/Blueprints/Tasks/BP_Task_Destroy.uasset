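; BP_Task_Destroy is a task actor that completes when damage depletes its health.
; An init interface call stores the EnemySpawner, and each hit lowers TaskHealth and updates the CaptureBar widget through an interface message.
; At zero health it notifies the spawner of completion and destroys itself.
; Capture-point logic with overlap and timer handling remains in the graph but is disconnected, leaving those events empty.
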(event OnComponentBeginOverlap(Collision)
  (params (OverlappedComponent :type Primitive%20Component%20Object%20Reference) (OtherActor :type Actor%20Object%20Reference) (OtherComp :type Primitive%20Component%20Object%20Reference) (OtherBodyIndex :type Integer) (bFromSweep :type Boolean) (SweepResult :type Hit%20Result%20Structure%20%28by%20ref%29))
  ;[0 0.7893 1] capture task logic
)

(event OnComponentEndOverlap(Collision)
  (params (OverlappedComponent :type Primitive%20Component%20Object%20Reference) (OtherActor :type Actor%20Object%20Reference) (OtherComp :type Primitive%20Component%20Object%20Reference) (OtherBodyIndex :type Integer))
  ;[0 0.7893 1] capture task logic
)

(event Custom|StartCapture
  ;[0 0.7893 1] capture task logic
)

(event Custom|StopCapture
  ;[0 0.7893 1] capture task logic
)

(event EventBeginPlay
  ;[1 1 0] Damage Task Logic
  (Class|BPITaskInterface|IDestroyTask(Message) (UserInterface|GetUserWidgetObject (Variables|Default|GetCapture_Bar)) (Variables|Default|GettaskHealth) (Variables|Default|GetMaxHealth)))

(event EventITaskInit
  (params (enemySpawner :type Enemy%20Spawner%20Object%20Reference))
  ;[1 1 1] should be in base task
  (Variables|Default|SetenemySpawner enemySpawner)
  (Variables|Default|Setcaptured false)
  (Variables|Default|SetcaptureAmount 0.0))

(event Game|Damage|EventAnyDamage
  (params (Damage :type Float%20%28single-precision%29) (DamageType :type Damage%20Type%20Object%20Reference) (InstigatedBy :type Controller%20Object%20Reference) (DamageCauser :type Actor%20Object%20Reference))
  ;[1 1 0] Damage Task Logic
  (Variables|Default|SettaskHealth (- (Variables|Default|GettaskHealth) Damage))
  (Class|BPITaskInterface|IDestroyTask(Message) (UserInterface|GetUserWidgetObject (Variables|Default|GetCapture_Bar)) (Variables|Default|GettaskHealth) (Variables|Default|GetMaxHealth))
  (if (<= (Variables|Default|GettaskHealth) 0.0)
    (Class|EnemySpawnerInterface|ITaskComplete(Message) (Variables|Default|GetenemySpawner))
    (Development|PrintString "Task Complete")
    (Actor|DestroyActor)))

(fn ConstructionScript)

(fn ITaskComplete
  (return 0.0))

(fn IIncreaseBar
  (return))