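; BP_Task_Capture is a capture-point task actor that fills while a player stands in its collision volume, then notifies the enemy spawner.
; Overlap starts a looping timer that accumulates capture progress and updates a widget bar via interface message; leaving stops the timer without resetting progress.
; Exceeding the required amount locks the point, changes its text and messages the spawner supplied through ITaskInit, which also resets capture state.
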(event OnComponentBeginOverlap(Collision)
  (params (OverlappedComponent :type Primitive%20Component%20Object%20Reference) (OtherActor :type Actor%20Object%20Reference) (OtherComp :type Primitive%20Component%20Object%20Reference) (OtherBodyIndex :type Integer) (bFromSweep :type Boolean) (SweepResult :type Hit%20Result%20Structure%20%28by%20ref%29))
  ;[0 0.7893 1] capture task logic
  (if (Utilities|DoesObjectImplementInterface OtherActor "/Game/Interface/playerInterface.playerInterface_C")
    (if (not (Variables|Default|Getcaptured))
      (bind _returnvalue (Utilities|Time|SetTimerbyEvent (EventDispatchers|CreateEvent :!event Custom|StartCapture) 0.1 true))
      (Variables|Default|SetTimer _returnvalue))))

(event OnComponentEndOverlap(Collision)
  (params (OverlappedComponent :type Primitive%20Component%20Object%20Reference) (OtherActor :type Actor%20Object%20Reference) (OtherComp :type Primitive%20Component%20Object%20Reference) (OtherBodyIndex :type Integer))
  ;[0 0.7893 1] capture task logic
  (if (Utilities|DoesObjectImplementInterface OtherActor "/Game/Interface/playerInterface.playerInterface_C")
    (if (not (Variables|Default|Getcaptured))
      (CallFunction|StopCapture))))

(event Custom|StartCapture
  ;[0 0.7893 1] capture task logic
  (Variables|Default|SetcaptureAmount (+ (Variables|Default|GetcaptureAmount) (Variables|Default|GetcaptureRate)))
  (Class|BPITaskInterface|ICapturePoint(Message) (UserInterface|GetUserWidgetObject (Variables|Default|GetCapture_Bar)) (Variables|Default|GetcaptureAmount) (Variables|Default|GetamountRequired))
  (if (> (Variables|Default|GetcaptureAmount) (Variables|Default|GetamountRequired))
    (CallFunction|StopCapture)
    (Variables|Default|Setcaptured true)
    (Rendering|Components|TextRender|SetText (Variables|Default|GetTextRender) (Variables|Default|GetdoneText))
    (Class|EnemySpawnerInterface|ITaskComplete(Message) (Variables|Default|GetenemySpawner))))

(event Custom|StopCapture
  (bind _timer (Variables|Default|GetTimer))
  ;[0 0.7893 1] capture task logic
  (Utilities|Time|PauseTimerbyHandle _timer)
  (Utilities|Time|ClearandInvalidateTimerbyHandle _timer))

(event EventBeginPlay)

(event EventITaskInit
  (params (enemySpawner :type Enemy%20Spawner%20Object%20Reference))
  ;[0.9122 0.4794 1] should be in base task
  (Variables|Default|SetenemySpawner enemySpawner)
  (Variables|Default|Setcaptured false)
  (Variables|Default|SetcaptureAmount 0.0))

(fn ConstructionScript)

(fn ITaskComplete
  (return 0.0))

(fn IIncreaseBar
  (return))