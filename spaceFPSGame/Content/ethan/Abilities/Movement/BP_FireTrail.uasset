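; BP_FireTrail is a short-lived fire hazard actor, filed under movement abilities, that despawns a few seconds after spawning.
; Overlapping its FireTrail component sends an ApplyFireStatus interface message to the other actor, applying timed damage per second.
; An array-based CheckandDamage pass, meant to skip actors touching multiple trails, is left disconnected: its array Add and its call never run.
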(event OnComponentBeginOverlap(FireTrail)
  (params (OverlappedComponent :type Primitive%20Component%20Object%20Reference) (OtherActor :type Actor%20Object%20Reference) (OtherComp :type Primitive%20Component%20Object%20Reference) (OtherBodyIndex :type Integer) (bFromSweep :type Boolean) (SweepResult :type Hit%20Result%20Structure%20%28by%20ref%29))
  ;[1 1 1] keeping it simple
  (Class|StatusEffectInterface|IApplyFireStatus(Message) OtherActor 2.0 2.0))

(event OnComponentEndOverlap(FireTrail)
  (params (OverlappedComponent :type Primitive%20Component%20Object%20Reference) (OtherActor :type Actor%20Object%20Reference) (OtherComp :type Primitive%20Component%20Object%20Reference) (OtherBodyIndex :type Integer))
  (Utilities|Array|RemoveItem (Variables|Default|GetActors%20Overlapping%20Fire%20Trail%20Array) OtherActor))

(event Custom|Check%20and%20Damage
  (for _array_element (Variables|Default|GetActors%20Overlapping%20Fire%20Trail%20Array)
    (if (not (>= (Utilities|Array|Length (Collision|GetOverlappingActors _array_element "BP_FireTrail_C" :!class /Script/Engine.Actor)) 2))
      (Class|StatusEffectInterface|IApplyFireStatus(Message) _array_element 1.0 6.0)
      (Development|PrintString (Utilities|String|Append "Damaging: " (Utilities|GetDisplayName _array_element))))))

(event EventBeginPlay
  ;[1 1 1] keeping it simple
  (Actor|SetLifeSpan 3.0))

(fn ConstructionScript)