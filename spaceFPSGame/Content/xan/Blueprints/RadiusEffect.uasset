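; RadiusEffect is an expanding sphere actor that applies a Burn or Freeze effect to actors it touches, then destroys itself.
; The construction script creates a dynamic material, which BeginPlay tints by effect type and makes translucent via a scalar parameter.
; A timeline scales the sphere from its starting scale to EndScale.
; Each newly overlapped actor receives a burn or freeze message with EffectDuration once, tracked in AffectedActors.
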(event OnComponentBeginOverlap(Sphere)
  (params (OverlappedComponent :type Primitive%20Component%20Object%20Reference) (OtherActor :type Actor%20Object%20Reference) (OtherComp :type Primitive%20Component%20Object%20Reference) (OtherBodyIndex :type Integer) (bFromSweep :type Boolean) (SweepResult :type Hit%20Result%20Structure%20%28by%20ref%29))
  (bind _effectduration (Variables|Default|GetEffectDuration))
  ;[1 1 1] Apply Effect on Overlap
  (if (not (Utilities|Array|ContainsItem (Variables|Default|GetAffectedActors) OtherActor))
    (switch Utilities|FlowControl|Switch|SwitchonEffectType (Variables|Default|GetType)
      (:NewEnumerator0
        (Class|StatusInterface|Burn(Message) OtherActor _effectduration))
      (:NewEnumerator1
        (Class|StatusInterface|Freeze(Message) OtherActor _effectduration)))
    (Utilities|Array|Add (Variables|Default|GetAffectedActors) OtherActor)))

(event EventBeginPlay
  (bind _matinst (Variables|Default|GetMatInst))
  (Utilities|FlowControl|Sequence
    (:then_0
      ;[1 1 1] Set Starting Scale
      (Variables|Default|SetStartScale (Transformation|GetActorScale3D)))
    (:then_1
      ;[1 1 1] Set material depending on effect type
      (switch Utilities|FlowControl|Switch|SwitchonEffectType (Variables|Default|GetType)
        (:NewEnumerator0
          (Rendering|Material|SetVectorParameterValue _matinst "DiffuseColor" "(R=1.000000,G=0.150000,B=0.000000,A=1.000000)" :!class /Script/Engine.MaterialInstanceDynamic))
        (:NewEnumerator1
          (Rendering|Material|SetVectorParameterValue _matinst "DiffuseColor" "(R=0.000000,G=0.850000,B=1.000000,A=1.000000)" :!class /Script/Engine.MaterialInstanceDynamic)))
      (Rendering|Material|SetScalarParameterValue _matinst "Occupacity" 0.25 :!class /Script/Engine.MaterialInstanceDynamic))
    (:then_2
      ;[1 1 1] Expand Radius of Effect
      (bind _alphatime (Timeline|Expand%20Radius Play)
        (:Update
          (Transformation|SetWorldScale3D (Variables|Default|GetSphere) (Math|Vector|Lerp(Vector) (Variables|Default|GetStartScale) (Variables|Default|GetEndScale) _alphatime)))
        (:Finished
          (Actor|DestroyActor))))))

(fn ConstructionScript
  (bind _returnvalue (Rendering|Material|CreateDynamicMaterialInstance (Variables|Default|GetSphere) 0 "/Game/xan/Materials/M_Base.M_Base" "None" :!class /Script/Engine.PrimitiveComponent))
  (Variables|Default|SetMatInst _returnvalue))