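; Elemental ground pool actor that periodically applies Fire burn or Ice freeze status to the actors inside it.
; On BeginPlay it tints its translucent dynamic material, grows the mesh to pool size via a timeline, and starts a looping tick timer.
; Collision overlaps maintain the list of affected actors, which receive status through interface messages on each tick.
; The pool destroys itself once its tick count runs out.
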(event OnComponentBeginOverlap(PoolCollision)
  (params (OverlappedComponent :type Primitive%20Component%20Object%20Reference) (OtherActor :type Actor%20Object%20Reference) (OtherComp :type Primitive%20Component%20Object%20Reference) (OtherBodyIndex :type Integer) (bFromSweep :type Boolean) (SweepResult :type Hit%20Result%20Structure%20%28by%20ref%29))
  ;[0 1 0.3] Store actors in the pool
  (Utilities|Array|AddUnique (Variables|Default|GetTouchingActors) OtherActor))

(event OnComponentEndOverlap(PoolCollision)
  (params (OverlappedComponent :type Primitive%20Component%20Object%20Reference) (OtherActor :type Actor%20Object%20Reference) (OtherComp :type Primitive%20Component%20Object%20Reference) (OtherBodyIndex :type Integer))
  ;[0 1 0.3] Store actors in the pool
  (Utilities|Array|RemoveItem (Variables|Default|GetTouchingActors) OtherActor))

(event Custom|Expand%20Pool
  (bind _poolmesh (Variables|Default|GetPoolMesh))
  (bind _poolsize (Variables|Default|GetPoolSize))
  ;[0 1 0.3] Scale pool to defined size
  (bind _alphatime (Timeline|Expand Play)
    (:Update
      (Transformation|SetWorldScale3D _poolmesh (Math|Vector|Lerp(Vector) (Transformation|GetWorldScale _poolmesh) (Math|Vector|MakeVector _poolsize _poolsize 0.1) _alphatime)))))

(event Custom|Damage%20Actors%20In%20Pool
  (bind _firevalues (Variables|Default|GetFireValues))
  ;[0 1 0.3] Apply a tick of damage to actors in the pool
  (if (> (Variables|Default|GetPoolTickAmount) 0)
    (Math|Integer|DecrementInt (Variables|Default|GetPoolTickAmount)
      (:%20%20
        (for _array_element (Variables|Default|GetTouchingActors)
          (Utilities|IsValid _array_element
            (:Is%20Valid
              (switch Utilities|FlowControl|Switch|SwitchonElementType (Variables|Default|GetElement)
                (:NewEnumerator0
                  (Class|StatusEffectInterface|IApplyFireStatus(Message) _array_element (.damagepersecond _firevalues) (.duration _firevalues)))
                (:NewEnumerator1
                  (Class|StatusEffectInterface|IApplyFreezeStatus(Message) _array_element (.staggerduration (Variables|Default|GetIceValues))))))))))
    (else
      ;[0 1 0.3] Destroy pool actor after final tick
      (Actor|DestroyActor))))

(event Custom|SetPoolColour
  (bind _matinst (Variables|Default|GetMatInst))
  (bind _colour (Variables|Default|GetColour))
  ;[0 1 0.3] Set pool colour
  (switch Utilities|FlowControl|Switch|SwitchonElementType (Variables|Default|GetElement)
    (:NewEnumerator0
      (Rendering|Material|SetVectorParameterValue _matinst "DiffuseColor" _colour :!class /Script/Engine.MaterialInstanceDynamic))
    (:NewEnumerator1
      (Rendering|Material|SetVectorParameterValue _matinst "DiffuseColor" _colour :!class /Script/Engine.MaterialInstanceDynamic)))
  (Rendering|Material|SetScalarParameterValue _matinst "Opacity" 0.25 :!class /Script/Engine.MaterialInstanceDynamic))

(event EventBeginPlay
  (Utilities|FlowControl|Sequence
    (:then_0
      (CallFunction|SetPoolColour))
    (:then_1
      (CallFunction|ExpandPool))
    (:then_2
      (Utilities|Time|SetTimerbyEvent (delegate Custom|Damage%20Actors%20In%20Pool) (Variables|Default|GetPoolTickInterval) true))))

(fn ConstructionScript
  (bind _returnvalue (Rendering|Material|CreateDynamicMaterialInstance (Variables|Default|GetPoolMesh) 0 "/Game/Materials/M_Base.M_Base" "None" :!class /Script/Engine.PrimitiveComponent))
  (Variables|Default|SetMatInst _returnvalue))

(fn IModifyMoveSpeed
  (params (Duration :type Float%20%28single-precision%29) (Percentage :type Float%20%28single-precision%29))
  (return 0.0))