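; FlamePool is an ability hazard actor that damages actors standing in it over time.
; On BeginPlay a timeline grows the pool mesh toward a flat disc of PoolSize, while overlap events track the actors touching it.
; A looping timer applies TickDamage to each valid tracked actor, counting down TickAmount and destroying the pool on the timer call after the final tick.
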(event OnComponentBeginOverlap(PoolCollision)
  (params (OverlappedComponent :type Primitive%20Component%20Object%20Reference) (OtherActor :type Actor%20Object%20Reference) (OtherComp :type Primitive%20Component%20Object%20Reference) (OtherBodyIndex :type Integer) (bFromSweep :type Boolean) (SweepResult :type Hit%20Result%20Structure%20%28by%20ref%29))
  ;[0 1 0.3] Store actors in the pool
  (Utilities|Array|AddUnique (Variables|Default|GetTouchingActors) OtherActor))

(event OnComponentEndOverlap(PoolCollision)
  (params (OverlappedComponent :type Primitive%20Component%20Object%20Reference) (OtherActor :type Actor%20Object%20Reference) (OtherComp :type Primitive%20Component%20Object%20Reference) (OtherBodyIndex :type Integer))
  ;[0 1 0.3] Store actors in the pool
  (Utilities|Array|RemoveItem (Variables|Default|GetTouchingActors) OtherActor))

(event Custom|Expand%20Pool
  (bind _poolmesh (Variables|Default|GetPoolMesh))
  (bind _poolsize (Variables|Default|GetPoolSize))
  ;[0 1 0.3] Scale pool to defined size
  (bind _alphatime (Timeline|Expand Play)
    (:Update
      (Transformation|SetWorldScale3D _poolmesh (Math|Vector|Lerp(Vector) (Transformation|GetWorldScale _poolmesh) (Math|Vector|MakeVector _poolsize _poolsize 0.1) _alphatime)))))

(event Custom|Damage%20Actors%20In%20Pool
  ;[0 1 0.3] Apply a tick of damage to actors in the pool
  (if (> (Variables|Default|GetTickAmount) 0)
    (Math|Integer|DecrementInt (Variables|Default|GetTickAmount)
      (:%20%20
        (for _array_element (Variables|Default|GetTouchingActors)
          (Utilities|IsValid _array_element
            (:Is%20Valid
              (Game|Damage|ApplyDamage _array_element (Variables|Default|GetTickDamage) 0 0))))))
    (else
      ;[0 1 0.3] Destroy pool actor after final tick
      (Actor|DestroyActor))))

(event EventBeginPlay
  (CallFunction|ExpandPool)
  (Utilities|Time|SetTimerbyEvent (delegate Custom|Damage%20Actors%20In%20Pool) (Variables|Default|GetTickInterval) true))

(fn ConstructionScript)