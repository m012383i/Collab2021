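; RadiusEffect is an expanding elemental pool ability that damages actors it touches and applies a status effect.
; On BeginPlay a timeline grows the mesh to its end scale, then another fades its tinted dynamic material before the actor destroys itself.
; Overlaps send damage through interface messages, then switch on Element to apply fire, freeze, toxic or electric status.
; An AffectedActors list limits each actor to one hit.
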(event OnComponentBeginOverlap(PoolMesh)
  (params (OverlappedComponent :type Primitive%20Component%20Object%20Reference) (OtherActor :type Actor%20Object%20Reference) (OtherComp :type Primitive%20Component%20Object%20Reference) (OtherBodyIndex :type Integer) (bFromSweep :type Boolean) (SweepResult :type Hit%20Result%20Structure%20%28by%20ref%29))
  (bind _firevalues (Variables|Default|GetFireValues))
  (bind _toxicvalues (Variables|Default|GetToxicValues))
  (bind _electricvalues (Variables|Default|GetElectricValues))
  ;[0 1 0.3] Apply element effect to actors within the pool
  (if (not (Utilities|Array|ContainsItem (Variables|Default|GetAffectedActors) OtherActor))
    (Class|DamageableInterface|IDamage(Message) OtherActor (Variables|Default|GetDamage))
    (switch Utilities|FlowControl|Switch|SwitchonElementType (Variables|Default|GetElement)
      (:NewEnumerator0
        (Class|StatusEffectInterface|IApplyFireStatus(Message) OtherActor (.damagepersecond _firevalues) (.duration _firevalues)))
      (:NewEnumerator1
        (Class|StatusEffectInterface|IApplyFreezeStatus(Message) OtherActor (.staggerduration (Variables|Default|GetIceValues))))
      (:NewEnumerator2
        (Class|StatusEffectInterface|IApplyToxicStatus(Message) OtherActor (.damageperseocnd _toxicvalues) (.duration _toxicvalues) (.spreadrange _toxicvalues)))
      (:NewEnumerator4
        (Class|StatusEffectInterface|IApplyElectricStatus(Message) OtherActor (.damage _electricvalues) (.chargeperhit _electricvalues))))
    (Utilities|Array|Add (Variables|Default|GetAffectedActors) OtherActor)))

(event EventBeginPlay
  (bind _matinst (Variables|Default|GetMatInst))
  (Utilities|FlowControl|Sequence
    (:then_0
      ;[0 1 0.3] Set starting scale
      (Variables|Default|SetStartScale (Transformation|GetActorScale3D)))
    (:then_1
      ;[0 1 0.3] Set material colour & opactiy
      (Rendering|Material|SetVectorParameterValue _matinst "DiffuseColor" (Variables|Default|GetColour) :!class /Script/Engine.MaterialInstanceDynamic)
      (Rendering|Material|SetScalarParameterValue _matinst "Opacity" 0.25 :!class /Script/Engine.MaterialInstanceDynamic))
    (:then_2
      ;[0 1 0.3] Expand pool to end scale
      (bind _alphatime (Timeline|Expand%20Radius Play)
        (:Update
          (Transformation|SetWorldScale3D (Variables|Default|GetPoolMesh) (Math|Vector|Lerp(Vector) (Variables|Default|GetStartScale) (Variables|Default|GetEndScale) _alphatime)))
        (:Finished
          ;[0 1 0.3] Fade out pool
          (bind _alphafade (Timeline|Fade%20Out Play)
            (:Update
              (Rendering|Material|SetScalarParameterValue (Variables|Default|GetMatInst) "Opacity" _alphafade :!class /Script/Engine.MaterialInstanceDynamic))
            (:Finished
              ;[0 1 0.3] Destroy actor
              (Actor|DestroyActor))))))))

(fn ConstructionScript
  (bind _returnvalue (Rendering|Material|CreateDynamicMaterialInstance (Variables|Default|GetPoolMesh) 0 "/Game/Materials/M_Base.M_Base" "None" :!class /Script/Engine.PrimitiveComponent))
  (Variables|Default|SetMatInst _returnvalue))