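; Temporary elemental turret that shoots nearby Damageable actors and destroys itself when its lifetime ends.
; Detection range overlaps maintain a target list, refocusing on the nearest and starting or stopping a looping fire timer through a DoOnce.
; Tick smoothly rotates the head toward the focused target.
; Shots are debug-drawn line traces along the barrel, sending damage plus a Fire, Ice, Toxic or Electric status through interface messages.
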(event OnComponentBeginOverlap(DetectionRange)
  (params (OverlappedComponent :type Primitive%20Component%20Object%20Reference) (OtherActor :type Actor%20Object%20Reference) (OtherComp :type Primitive%20Component%20Object%20Reference) (OtherBodyIndex :type Integer) (bFromSweep :type Boolean) (SweepResult :type Hit%20Result%20Structure%20%28by%20ref%29))
  ;[0 1 0.3] Target Detection
  (if (Utilities|DoesObjectImplementInterface OtherActor "/Game/Interface/DamageableInterface.DamageableInterface_C")
    (Utilities|Array|AddUnique (Variables|Default|GetTargetsWithinRange) OtherActor)
    (CallFunction|CheckforValidTarget)))

(event OnComponentEndOverlap(DetectionRange)
  (params (OverlappedComponent :type Primitive%20Component%20Object%20Reference) (OtherActor :type Actor%20Object%20Reference) (OtherComp :type Primitive%20Component%20Object%20Reference) (OtherBodyIndex :type Integer))
  ;[0 1 0.3] Target Detection
  (Utilities|Array|RemoveItem (Variables|Default|GetTargetsWithinRange) OtherActor)
  (CallFunction|CheckforValidTarget))

(event Custom|Check%20For%20Valid%20Target
  ;[0 1 0.3] Check if there are any valid targets in the array
  (if (!= (Utilities|Array|LastIndex (Variables|Default|GetTargetsWithinRange)) -1)
    ;[0 1 0.3] Set the nearest target in that array as the focused target
    (bind _nearesttarget (CallFunction|FindNearestTarget (Variables|Default|GetTargetsWithinRange)))
    (Variables|Default|SetFocusedTarget _nearesttarget)
    ;[0 1 0.3] Start attacking the focused target
    (Utilities|FlowControl|DoOnce false :!label _label
      (:Completed
        (bind _returnvalue (Utilities|Time|SetTimerbyFunctionName 0 "FireShot" (Variables|Default|GetShotInterval) true))
        (Variables|Default|SetTimerHandle _returnvalue)))
    (else
      ;[0 1 0.3] Stop attacking if there are no valid targets
      (Utilities|Time|ClearandInvalidateTimerbyHandle (Variables|Default|GetTimerHandle))
      (Variables|Default|SetFocusedTarget 0)
      (goto _label Reset))))

(event Custom|Aim%20At%20Target
  (bind _head (Variables|Default|GetHead))
  (bind _focusedtarget (Variables|Default|GetFocusedTarget))
  (bind _returnvalue (Transformation|GetWorldLocation _head))
  (bind _returnvalue_2 (Transformation|GetActorLocation _focusedtarget))
  (bind _returnvalue_3 (Math|Rotator|FindLookatRotation _returnvalue _returnvalue_2))
  (bind (_roll _pitch _yaw) (Math|Rotator|BreakRotator _returnvalue_3))
  ;[0 1 0.3] Rotate turret toward focused target
  (Utilities|IsValid _focusedtarget
    (:Is%20Valid
      (Transformation|SetWorldRotation _head (Math|Interpolation|RInterpTo (Transformation|GetWorldRotation _head) (Math|Rotator|MakeRotator 0.0 _pitch _yaw) (Variables|Default|GetDeltaTime) (Variables|Default|GetRotationSpeed)) false false))))

(event EventBeginPlay
  ;[0 1 0.3] Destroy turret after lifetime duration elapsed
  (Utilities|FlowControl|Delay (Variables|Default|GetLifetime))
  (Actor|DestroyActor))

(event EventTick
  (params (DeltaSeconds :type Float%20%28single-precision%29))
  (Variables|Default|SetDeltaTime DeltaSeconds)
  (CallFunction|AimatTarget))

(fn ConstructionScript)

(fn FindNearestTarget
  (params (TargetsToSearch :type Array%20of%20Actor%20Object%20References))
  (for (_array_element _array_index) TargetsToSearch
    (if (<= _array_index 0)
      (bind _output_get (LocalVariables|SetCurClosestDist (Transformation|GetDistanceTo _array_element)))
      (LocalVariables|SetCurClosestTarget _array_element :!label _label)
      (elif (> _output_get (Transformation|GetDistanceTo _array_element))
        (LocalVariables|SetCurClosestDist (Transformation|GetDistanceTo _array_element))
        (goto _label))))
  (return (LocalVariables|GetCurClosestTarget)))

(fn FireShot
  (bind _barreldirection (Variables|Default|GetBarrelDirection))
  (bind _firevalues (Variables|Default|GetFireValues))
  (bind _toxicvalues (Variables|Default|GetToxicValues))
  (bind _electricvalues (Variables|Default|GetElectricValues))
  (bind _returnvalue (Transformation|GetWorldLocation _barreldirection))
  (bind (_outhit _returnvalue_2) (Collision|LineTraceByChannel _returnvalue (+ _returnvalue (* (Math|Vector|GetForwardVector _barreldirection) (Variables|Default|GetShotRange))) "TraceTypeQuery1" false (Utilities|Array|MakeArray self) "ForDuration" true "(R=1.000000,G=0.833333,B=0.000000,A=1.000000)" "(R=0.000000,G=1.000000,B=0.000000,A=1.000000)" 0.2))
  (if (and _returnvalue_2 (Utilities|DoesObjectImplementInterface (.HitActor (Collision|BreakHitResult _outhit)) "/Game/Interface/DamageableInterface.DamageableInterface_C"))
    (Class|DamageableInterface|IDamage(Message) (.HitActor (Collision|BreakHitResult _outhit)) (Variables|Default|GetShotDamage))
    (switch Utilities|FlowControl|Switch|SwitchonElementType (Variables|Default|GetElement)
      (:NewEnumerator0
        (Class|StatusEffectInterface|IApplyFireStatus(Message) (.HitActor (Collision|BreakHitResult _outhit)) (.damagepersecond _firevalues) (.duration _firevalues)))
      (:NewEnumerator1
        (Class|StatusEffectInterface|IApplyFreezeStatus(Message) (.HitActor (Collision|BreakHitResult _outhit)) (.staggerduration (Variables|Default|GetIceValues))))
      (:NewEnumerator2
        (Class|StatusEffectInterface|IApplyToxicStatus(Message) (.HitActor (Collision|BreakHitResult _outhit)) (.damageperseocnd _toxicvalues) (.duration _toxicvalues) (.spreadrange _toxicvalues)))
      (:NewEnumerator4
        (Class|StatusEffectInterface|IApplyElectricStatus(Message) (.HitActor (Collision|BreakHitResult _outhit)) (.damage _electricvalues) (.chargeperhit _electricvalues))))))