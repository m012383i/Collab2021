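; GM_SpaceFPS is the game mode for a space FPS, tracking pause state and room-clear progression.
; Interface calls toggle pause, switch between the game and main menu maps with explicit game modes, and expose state to callers.
; Each cleared room increments the count and linearly raises the enemy stats multiplier, and the last-room check is true whenever the count is a multiple of six, including zero.
; BeginPlay starts the ambient track.
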(event EventBeginPlay
  ;[0.9191 1 0] Ambient Track
  (Audio|PlaySound2D "/Game/Sound_Liam_/Ambient/Ambient_Track.Ambient_Track" 1.0 1.0 0.0 0 0))

(event EventIGMIncreaseRoomNumber
  ;[0 0.9911 1] increase room clear number
  (Math|Integer|IncrementInt (Variables|Default|GetroomsCleared)
    (:%20%20
      (Variables|Default|SetenemyStatsMultiplier (+ (Variables|Default|GetenemyStatsMultiplier) (Variables|Default|GetstatsIncreaseRate))))))

(event EventIGMLoadGameMap
  ;[0 0.9911 1] load game map
  (Game|OpenLevel(byName) "Testmap" true (Utilities|String|Append "?game=" "/Game/michael/GM_SpaceFPS.GM_SpaceFPS_C")))

(event EventIGMResumeGame
  ;[0 0.9911 1] pause and resume
  (bind _returnvalue (Game|SetGamePaused false))
  (Variables|Default|SetisGamePaused _returnvalue)
  (Variables|Default|SetgameModeState "NewEnumerator0"))

(event EventIGMPauseGame
  ;[0 0.9911 1] pause and resume
  (bind _returnvalue (Game|SetGamePaused true))
  (Variables|Default|SetisGamePaused _returnvalue)
  (Variables|Default|SetgameModeState "NewEnumerator1"))

(event EventIGMLoadMenu
  ;[0 0.9911 1] load main menu map
  (Game|OpenLevel(byName) "EthanMainMenu" true (Utilities|String|Append "?game=" "/Game/ethan/MenuWidgets/GM_MainMenu.GM_MainMenu_C")))

(fn ConstructionScript)

(fn IGMGetEnemyMultiplier
  ;[0 0.9911 1] getting the enemy stats multiplier
  (return (Variables|Default|GetenemyStatsMultiplier)))

(fn IGMGetRoomsCleared
  (return (Variables|Default|GetroomsCleared)))

(fn IGMIsatLastRoom
  (return (not (> (.Remainder (Math|Float|Division(WholeandRemainder) (Math|Conversions|ToFloat(Integer) (Variables|Default|GetroomsCleared)) 6.0)) 0.0))))

(fn IGMIsGamePaused
  (return (Variables|Default|GetisGamePaused)))